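; Bomberman board Blueprint that drives the game-over screen for a match between a blue and an orange player.
; Every Tick it checks IsTheGameOver and compares Winner to each player to pick a blue win, orange win or tie message.
; It finds the existing GameOverWidget by class each frame and writes its title, winner message and restart instructions directly, blanking all three while play continues.
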(event `self.ReceiveTick`
  (params (DeltaSeconds :type "Float (single-precision)"))
  (bind _returnvalue (`KismetTextLibrary.Conv_TextToString` (`KismetTextLibrary.GetEmptyText`)))
  (bind _returnvalue_2 (`self.IsTheGameOver`))
  (if _returnvalue_2
    (if (== (`self.BluePlayer`) (`self.winner`))
      ;[1 1 1] Game over GUI w/ blue player as the winner
      (bind _foundwidgets (`WidgetBlueprintLibrary.GetAllWidgetsOfClass` "/Game/Screens/GameOverWidget.GameOverWidget_C"))
      (bind _asgame_over_widget (cast `/Game/Screens/GameOverWidget` (`|GetArrayItem` _foundwidgets)))
      (`|ExecutionSequence`
        (:`then_0`
          (set `/Game/Screens/GameOverWidget.GameOverTitle` (`self.GameOverTitle`) _asgame_over_widget))
        (:`then_1`
          (set `/Game/Screens/GameOverWidget.RestartInstructions` (`self.RestartInstructions`) _asgame_over_widget))
        (:`then_2`
          (set `/Game/Screens/GameOverWidget.PlayerWinMessage` (`self.BluePlayerName`) _asgame_over_widget)))
      (elif (== (`self.OrangePlayer`) (`self.winner`))
        ;[1 1 1] Game over GUI w/ orange player as the winner
        (bind _foundwidgets_2 (`WidgetBlueprintLibrary.GetAllWidgetsOfClass` "/Game/Screens/GameOverWidget.GameOverWidget_C"))
        (bind _asgame_over_widget_2 (cast `/Game/Screens/GameOverWidget` (`|GetArrayItem` _foundwidgets_2)))
        (`|ExecutionSequence`
          (:`then_0`
            (set `/Game/Screens/GameOverWidget.GameOverTitle` (`self.GameOverTitle`) _asgame_over_widget_2))
          (:`then_1`
            (set `/Game/Screens/GameOverWidget.RestartInstructions` (`self.RestartInstructions`) _asgame_over_widget_2))
          (:`then_2`
            (set `/Game/Screens/GameOverWidget.PlayerWinMessage` (`self.OrangePlayerName`) _asgame_over_widget_2)))
        (else
          ;[1 1 1] Game over GUI w/ no winner
          (bind _foundwidgets_3 (`WidgetBlueprintLibrary.GetAllWidgetsOfClass` "/Game/Screens/GameOverWidget.GameOverWidget_C"))
          (bind _asgame_over_widget_3 (cast `/Game/Screens/GameOverWidget` (`|GetArrayItem` _foundwidgets_3)))
          (`|ExecutionSequence`
            (:`then_0`
              (set `/Game/Screens/GameOverWidget.GameOverTitle` (`self.GameOverTitle`) _asgame_over_widget_3))
            (:`then_1`
              (set `/Game/Screens/GameOverWidget.RestartInstructions` (`self.RestartInstructions`) _asgame_over_widget_3))
            (:`then_2`
              (set `/Game/Screens/GameOverWidget.PlayerWinMessage` (`self.Tie`) _asgame_over_widget_3))))))
    (else
      ;[1 1 1] Empty GUI while the game is not over
      (bind _foundwidgets_4 (`WidgetBlueprintLibrary.GetAllWidgetsOfClass` "/Game/Screens/GameOverWidget.GameOverWidget_C"))
      (bind _asgame_over_widget_4 (cast `/Game/Screens/GameOverWidget` (`|GetArrayItem` _foundwidgets_4)))
      (`|ExecutionSequence`
        (:`then_0`
          (set `/Game/Screens/GameOverWidget.PlayerWinMessage` _returnvalue _asgame_over_widget_4))
        (:`then_1`
          (set `/Game/Screens/GameOverWidget.RestartInstructions` _returnvalue _asgame_over_widget_4))
        (:`then_2`
          (set `/Game/Screens/GameOverWidget.GameOverTitle` _returnvalue _asgame_over_widget_4))))))

(fn `UserConstructionScript`)